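; Green Viking AI enemy character for a VR combat game, with montage-driven attacks and selectable movement speeds.
; Capsule overlaps with the player's weapon collision count hits until a threshold switches the Blackboard AI state.
; That threshold also checks the player's kill total, showing a win widget and loading Game_WP once the target is reached.
; Attack halts movement and signals attack end; patrol, tag and task-state functions are stubs.
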(event OnComponentBeginOverlap(CapsuleComponent)
  (params (OverlappedComponent :type Primitive%20Component%20Object%20Reference) (OtherActor :type Actor%20Object%20Reference) (OtherComp :type Primitive%20Component%20Object%20Reference) (OtherBodyIndex :type Integer) (bFromSweep :type Boolean) (SweepResult :type Hit%20Result%20Structure%20%28by%20ref%29))
  ;[1 1 1] Comment
  (bind _asvrpawn (Utilities|Casting|CastToVRPawn OtherActor))
  (if (Class|PrimitiveComponent|IsOverlappingComponent (Variables|Collision|GetCapsuleComponent self) (Variables|/Game/VRTemplate/Blueprints/VRPawn.VRPawn_C|GetWeapon%20Collision _asvrpawn))
    (if (>= (Variables|Default|GetHitsToKill) 2)
      (Variables|Default|SetHitsToKill 0)
      (AI|Components|Blackboard|SetValueasEnum (AI|GetBlackboard self) (Variables|Default|GetKey%20Name) (Utilities|Enum|LiteralenumE_AIState "NewEnumerator4"))
      (bind _asvrpawn_2 (Utilities|Casting|CastToVRPawn (Game|Player|GetPlayerPawn 0)))
      (if (not (< (Variables|/Game/VRTemplate/Blueprints/VRPawn.VRPawn_C|GetKills _asvrpawn_2) 50))
        (bind _returnvalue (UserInterface|CreateWidget "/Game/UI/WinUi.WinUI_C"))
        (UserInterface|SetWidget (Variables|/Game/VRTemplate/Blueprints/VRPawn.VRPawn_C|GetHUD _asvrpawn_2) _returnvalue)
        (Utilities|FlowControl|Delay 3.0)
        (Game|OpenLevel(byName) "Game_WP"))
      (else
        (Math|Integer|IncrementInt (Variables|Default|GetHitsToKill))))))

(event Custom|Attack
  (Components|Movement|StopMovementImmediately (Variables|Character|GetCharacterMovement))
  (Animation|Montage|PlayMontage (Variables|Character|GetMesh) "/Game/Animations/GreenViking/Attack_GreenViking_AnimMontage.Attack_GreenViking_AnimMontage"
    (:OnCompleted
      _)
    (:OnInterrupted
      _))
  (Default|CallOnAttackEnd))

(fn ConstructionScript)

(fn GetPatrolRoute
  (return 0))

(fn SelectTag
  (params (NewParam :type E_TaskUse%20Enum :default "NewEnumerator1"))
  (return "None"))

(fn SetMovementSpeed
  (params (Speed :type E_MovementSpeed%20Enum :default "NewEnumerator0"))
  (Variables|/Script/Engine.CharacterMovementComponent|SetMaxWalkSpeed (Variables|Character|GetCharacterMovement) (Utilities|Select :Index Speed :NewEnumerator0 0.0 :NewEnumerator1 1e+02 :NewEnumerator2 2.5e+02 :NewEnumerator3 3.5e+02))
  (return 0.0))

(fn SetTaskState
  (params (Task :type E_TaskUse%20Enum :default "NewEnumerator1"))
  (return false))