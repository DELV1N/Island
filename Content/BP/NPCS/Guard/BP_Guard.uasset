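; BP_Guard is a guard NPC that takes a set number of hits to kill and can trigger the game win.
; Each capsule overlap waits five seconds, then decrements HitsToKill or, if already depleted, destroys the guard.
; After destruction it checks VRPawn's kill count, which it never increments, and at the threshold shows WinUI before reloading "Game" via a delay.
; Patrol, tag, speed and task-state functions are empty stubs.
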(event OnComponentBeginOverlap(CapsuleComponent)
  (params (OverlappedComponent :type Primitive%20Component%20Object%20Reference) (OtherActor :type Actor%20Object%20Reference) (OtherComp :type Primitive%20Component%20Object%20Reference) (OtherBodyIndex :type Integer) (bFromSweep :type Boolean) (SweepResult :type Hit%20Result%20Structure%20%28by%20ref%29))
  (bind _returnvalue (Game|Player|GetPlayerPawn 0))
  (Utilities|FlowControl|Delay 5.0)
  (if (<= (Variables|Default|GetHitsToKill) 0)
    (Actor|DestroyActor)
    (bind _asvrpawn (Utilities|Casting|CastToVRPawn _returnvalue))
    (if (not (< (Variables|/Game/VRTemplate/Blueprints/VRPawn.VRPawn_C|GetKills _asvrpawn) 50))
      (bind _asvrpawn_2 (Utilities|Casting|CastToVRPawn _returnvalue))
      (bind _returnvalue_2 (UserInterface|CreateWidget "/Game/UI/WinUi.WinUI_C"))
      (UserInterface|SetWidget (Variables|/Game/VRTemplate/Blueprints/VRPawn.VRPawn_C|GetHUD _asvrpawn_2) _returnvalue_2)
      (Utilities|FlowControl|Delay 3.0)
      (Game|OpenLevel(byName) "Game"))
    (else
      (Variables|Default|SetHitsToKill (- (Variables|Default|GetHitsToKill) 1)))))

(fn ConstructionScript)

(fn GetPatrolRoute
  (return 0))

(fn SelectTag
  (params (NewParam :type E_TaskUse%20Enum :default "NewEnumerator1"))
  (return "None"))

(fn SetMovementSpeed
  (params (Speed :type E_MovementSpeed%20Enum :default "NewEnumerator0"))
  (return 0.0))

(fn SetTaskState
  (params (Task :type E_TaskUse%20Enum :default "NewEnumerator1"))
  (return false))