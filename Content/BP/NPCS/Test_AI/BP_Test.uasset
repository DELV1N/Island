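; Test AI enemy NPC for the VR game, with a hit-count death and a Blue Viking attack montage.
; Capsule overlaps, after a delay, decrement HitsToKill or destroy the actor at zero, then check VRPawn's kill count to show the win UI and queue a Game level load.
; Attack signals its end on montage completion or interruption.
; Helpers expose the patrol route, movement speed presets and NotUsed/InUse task state, with NotUsed tagged on possession.
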(event OnComponentBeginOverlap(CapsuleComponent)
  (params (OverlappedComponent :type Primitive%20Component%20Object%20Reference) (OtherActor :type Actor%20Object%20Reference) (OtherComp :type Primitive%20Component%20Object%20Reference) (OtherBodyIndex :type Integer) (bFromSweep :type Boolean) (SweepResult :type Hit%20Result%20Structure%20%28by%20ref%29))
  (bind _returnvalue (Game|Player|GetPlayerPawn 0))
  ;[1 1 1] Default
  (Utilities|FlowControl|Delay 5.0)
  (if (<= (Variables|Default|GetHitsToKill) 0)
    (Actor|DestroyActor)
    (bind _asvrpawn (Utilities|Casting|CastToVRPawn _returnvalue))
    (if (not (< (Variables|/Game/VRTemplate/Blueprints/VRPawn.VRPawn_C|GetKills _asvrpawn) 50))
      (bind _asvrpawn_2 (Utilities|Casting|CastToVRPawn _returnvalue))
      (bind _returnvalue_2 (UserInterface|CreateWidget "/Game/UI/WinUi.WinUI_C"))
      (UserInterface|SetWidget (Variables|/Game/VRTemplate/Blueprints/VRPawn.VRPawn_C|GetHUD _asvrpawn_2) _returnvalue_2)
      (Utilities|FlowControl|Delay 3.0)
      (Game|OpenLevel(byName) "Game"))
    (else
      (Variables|Default|SetHitsToKill (- (Variables|Default|GetHitsToKill) 1)))))

(event Custom|Attack
  ;[1 1 1] Comment
  (Animation|Montage|PlayMontage (Variables|Character|GetMesh) "/Game/Animations/BlueViking/Attack_BlueViking_AnimMontage.Attack_BlueViking_AnimMontage"
    (:OnCompleted
      _)
    (:OnInterrupted
      _))
  (Default|CallOnAttackEnd))

(event EventPossessed
  (params (NewController :type Controller%20Object%20Reference))
  ;[1 1 1] OnStart (required)
  (Utilities|Array|Insert (Variables|Actor|GetTags) "NotUsed"))

(fn ConstructionScript)

(fn TaskSystem
  (return))

(fn GetPatrolRoute
  (return (Variables|Default|GetPatrolRoute)))

(fn SelectTag
  (params (NewParam :type E_TaskUse%20Enum :default "NewEnumerator1"))
  (if (Utilities|Select :Index NewParam :NewEnumerator1 false :NewEnumerator0 true)
    (return "InUse")
    (else
      (return "NotUsed"))))

(fn SetMovementSpeed
  (params (Speed :type E_MovementSpeed%20Enum :default "NewEnumerator0"))
  (bind _output_get (Variables|/Script/Engine.CharacterMovementComponent|SetMaxWalkSpeed (Variables|Character|GetCharacterMovement) (Utilities|Select :Index Speed :NewEnumerator0 0.0 :NewEnumerator1 1e+02 :NewEnumerator2 3e+02 :NewEnumerator3 3.5e+02)))
  (return _output_get))

(fn SetTaskState
  (params (Task :type E_TaskUse%20Enum :default "NewEnumerator1"))
  (return (Utilities|Select :Index Task :NewEnumerator1 false :NewEnumerator0 true)))