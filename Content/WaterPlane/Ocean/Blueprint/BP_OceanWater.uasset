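; BP_OceanWater is an ocean surface actor whose look is configured from Blueprint variables at construction time.
; The construction script creates a dynamic instance of OceanMaterial on WaterSurface and scales that component in X and Y.
; It then pushes speed, scale, displacement, tessellation and large and small wave amplification into the instance as scalar parameters.
; The graphs shown contain no runtime logic, leaving any wave motion to the material.
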(fn ConstructionScript
  (|InitialWaterCreation)
  (Rendering|Material|SetScalarParameterValue (Variables|Default|GetWater%20Material) "WaterSpeed" (Variables|Default|GetOverall%20Water%20Speed) :!class /Script/Engine.MaterialInstanceDynamic)
  (Rendering|Material|SetScalarParameterValue (Variables|Default|GetWater%20Material) "WaterScale" (Variables|Default|GetOverall%20Water%20Scale) :!class /Script/Engine.MaterialInstanceDynamic)
  (Rendering|Material|SetScalarParameterValue (Variables|Default|GetWater%20Material) "Displacement" (Variables|Default|GetDisplacement) :!class /Script/Engine.MaterialInstanceDynamic)
  (Rendering|Material|SetScalarParameterValue (Variables|Default|GetWater%20Material) "Tesselation" (Variables|Default|GetTesselation%20Factor) :!class /Script/Engine.MaterialInstanceDynamic)
  (Rendering|Material|SetScalarParameterValue (Variables|Default|GetWater%20Material) "Large Wave Amplify" (Variables|Default|GetAmplify%20Large%20Normals) :!class /Script/Engine.MaterialInstanceDynamic)
  (Rendering|Material|SetScalarParameterValue (Variables|Default|GetWater%20Material) "Small Wave Amplify" (Variables|Default|GetAmplify%20Small%20Normals) :!class /Script/Engine.MaterialInstanceDynamic))